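; Dialogue trigger volume that plays a 2D dialogue sound the first time BP_Chara enters its box.
; A DoOnce guards the playback, so later entries stay silent.
; When any overlap ends, it sets the Master sound class volume in the MasterVolume mix from the value stored in GI_Shen.
; A separate ShowDialogues event calls PlaySound2D with no sound assigned.
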(event OnComponentBeginOverlap(Box)
  (params (OverlappedComponent :type Primitive%20Component%20Object%20Reference) (OtherActor :type Actor%20Object%20Reference) (OtherComp :type Primitive%20Component%20Object%20Reference) (OtherBodyIndex :type Integer) (bFromSweep :type Boolean) (SweepResult :type Hit%20Result%20Structure%20%28by%20ref%29))
  (Utilities|Casting|CastToBP_Chara OtherActor)
  (Utilities|FlowControl|DoOnce false
    (:Completed
      (Audio|PlaySound2D (Variables|Default|GetDialogues) 1.0 1.0 0.0 0 0))))

(event OnComponentEndOverlap(Box)
  (params (OverlappedComponent :type Primitive%20Component%20Object%20Reference) (OtherActor :type Actor%20Object%20Reference) (OtherComp :type Primitive%20Component%20Object%20Reference) (OtherBodyIndex :type Integer))
  (bind _asgi_shen (Utilities|Casting|CastToGI_Shen (Game|GetGameInstance)))
  (Audio|SetSoundMixClassOverride "/Game/Spirit/Blueprints/Son/Mix/MasterVolume.MasterVolume" "/Engine/EngineSounds/Master.Master" (Variables|/Game/Spirit/Blueprints/Manager/GI_Shen.GI_Shen_C|GetMasterVolumeValue _asgi_shen) 1.0 1.0 true))

(event Custom|ShowDialogues
  (Audio|PlaySound2D 0 1.0 1.0 0.0 0 0))

(event EventBeginPlay)

(event Collision|EventActorBeginOverlap
  (params (OtherActor :type Actor%20Object%20Reference)))

(event EventTick
  (params (DeltaSeconds :type Float%20%28single-precision%29)))

(fn ConstructionScript)