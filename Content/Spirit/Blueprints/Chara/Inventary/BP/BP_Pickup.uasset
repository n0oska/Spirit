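; BP_Pickup is a world item pickup that a BP_Chara can collect with the interact input.
; Its ID looks up a DT_Inventory row on construction, BeginPlay and replication, setting the widget's name text and a skeletal mesh or fallback static mesh.
; Sphere overlap toggles the prompt and input for characters not locally AI-controlled.
; Interacting passes the item to the character's PickupItem, then destroys the pickup whatever the result.
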(event OnComponentBeginOverlap(Sphere)
  (params (OverlappedComponent :type Primitive%20Component%20Object%20Reference) (OtherActor :type Actor%20Object%20Reference) (OtherComp :type Primitive%20Component%20Object%20Reference) (OtherBodyIndex :type Integer) (bFromSweep :type Boolean) (SweepResult :type Hit%20Result%20Structure%20%28by%20ref%29))
  (bind _asbp_chara (Utilities|Casting|CastToBP_Chara OtherActor))
  (bind _isnpc (Utilities|IsPlayer _asbp_chara)
    (:True
      _)
    (:False
      (Rendering|SetVisibility (Variables|Default|GetWidget) true false)
      (Input|EnableInput (Game|GetPlayerController 0))
      (bind _output_get (Variables|Default|SetBP_Chara _asbp_chara))))
  (if (not _isnpc)
    (Actor|SetOwner _output_get)))

(event OnComponentEndOverlap(Sphere)
  (params (OverlappedComponent :type Primitive%20Component%20Object%20Reference) (OtherActor :type Actor%20Object%20Reference) (OtherComp :type Primitive%20Component%20Object%20Reference) (OtherBodyIndex :type Integer))
  (bind _asbp_chara (Utilities|Casting|CastToBP_Chara OtherActor))
  (Utilities|IsPlayer _asbp_chara
    (:False
      (Rendering|SetVisibility (Variables|Default|GetWidget) false false)
      (Input|DisableInput (Game|GetPlayerController 0))
      (Variables|Default|SetBP_Chara (stale OnComponentBeginOverlap(Sphere) _asbp_chara)))))

(event Custom|Update
  (bind _item (Variables|Default|GetItem))
  (bind (_displayname _pickupmesh _pickupmesh2) (Utilities|Struct|BreakST_InventoryItem _item))
  (bind _aswbp_pickup (Utilities|Casting|CastToWBP_Pickup (UserInterface|GetWidget (Variables|Default|GetWidget))))
  (Rendering|Components|TextRender|SetText (Variables|/Game/Spirit/Blueprints/Chara/Inventary/Widgets/WBP_Pickup.WBP_Pickup_C|Gettxt _aswbp_pickup) _displayname)
  (bind _returnvalue (Utilities|LoadAssetBlocking _pickupmesh))
  (bind _asskeletal_mesh (Utilities|Casting|CastToSkeletalMesh _returnvalue)
    (:then
      (Components|SkeletalMesh|SetSkeletalMeshAsset (Variables|Default|GetSkeletalMesh) _asskeletal_mesh))
    (:CastFailed
      (bind _returnvalue_2 (Utilities|LoadAssetBlocking _pickupmesh2))
      (bind _asstatic_mesh (Utilities|Casting|CastToStaticMesh _returnvalue_2))
      (Components|StaticMesh|SetStaticMesh (Variables|Default|GetStaticMesh) _asstatic_mesh))))

(event Custom|DestroyServer
  (Utilities|FlowControl|Delay 0.001)
  (Actor|DestroyActor))

(event Input|EnhancedActionEvents|EnhancedInputActionIA_Interact
  (params (ActionValue :type Boolean) (ElapsedSeconds :type Float%20%28double-precision%29) (TriggeredSeconds :type Float%20%28double-precision%29) (InputAction :type Input%20Action%20Object%20Reference :default "/Game/Spirit/Inputs/Input_Actions/IA_Interact.IA_Interact"))
  (bind _success (Default|PickupItem (Variables|Default|GetBP_Chara) (Variables|Default|GetID) (Variables|Default|GetItem)))
  (if _success
    (CallFunction|DestroyServer)
    (else
      (CallFunction|DestroyServer))))

(event EventBeginPlay
  (Components|StaticMesh|SetStaticMesh (Variables|Default|GetStaticMesh) "/Game/LevelPrototyping/Interactable/Target/Assets/SM_TargetBaseMesh.SM_TargetBaseMesh")
  (CallFunction|OnRepID))

(fn ConstructionScript
  (CallFunction|OnRepID))

(fn OnRepID
  (bind _returnvalue (Utilities|GetDataTableRow "/Game/Spirit/Blueprints/Chara/Inventary/DT_Inventory.DT_Inventory" (Variables|Default|GetID))
    (:then
      (Variables|Default|SetItem _returnvalue)
      (CallFunction|Update))))

(fn Interact
  (return "Interact_Object"))

(fn PickupItem
  (params (ID :type Name :default "None") (DropItem :type ST%20Inventory%20Item%20Structure))
  (return false))