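; Actor component that gives the player an inventory screen, toggled with the interact input.
; On BeginPlay it creates a BPW_inventary widget for the first player controller and stores it.
; IA_Interact removes the widget from the viewport if visible; otherwise it adds it and resizes the Items array to a fixed slot count.
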(event Input|EnhancedActionEvents|EnhancedInputActionIA_Interact
  (params (ActionValue :type Boolean) (ElapsedSeconds :type Float%20%28double-precision%29) (TriggeredSeconds :type Float%20%28double-precision%29) (InputAction :type Input%20Action%20Object%20Reference :default "/Game/Spirit/Inputs/Input_Actions/IA_Interact.IA_Interact"))
  (bind _wbp_inventory (Variables|Default|GetWBP_Inventory))
  (:Started
    (if (Widget|IsVisible _wbp_inventory)
      (Widget|RemovefromParent _wbp_inventory)
      (else
        (UserInterface|Viewport|AddtoViewport _wbp_inventory 0)
        (Utilities|Array|Resize (Variables|Default|GetItems) 10)))))

(event EventBeginPlay
  (bind _returnvalue (UserInterface|CreateWidget "/Game/Spirit/Blueprints/Chara/Inventary/Widgets/BPW_inventary.BPW_inventary_C" (Game|GetPlayerController 0)))
  (Variables|Default|SetWBP_Inventory _returnvalue))

(event EventTick
  (params (DeltaSeconds :type Float%20%28single-precision%29)))