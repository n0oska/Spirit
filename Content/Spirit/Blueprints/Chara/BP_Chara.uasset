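; Player character Blueprint for Spirit, with Enhanced Input movement, look, sprint, crouch, swimming, jump-glide and a cooldown-limited dash.
; Sprint, glide and dash drain a shared stamina resource that regenerates on timers, while gliding lowers gravity and raises air control.
; A per-tick camera trace finds BPI_Inventory actors for interaction, feeding objective calls alongside an inventory component.
; It also handles damage, GameMode-based respawn, pause menu and movement feedback; grab logic is disconnected.
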(event Custom|OnApexReached
  (bind _charactermovement (Variables|Character|GetCharacterMovement))
  (bind _charactermovement_2 (Variables|Character|GetCharacterMovement))
  (bind _charactermovement_3 (Variables|Character|GetCharacterMovement))
  ;[0.044 0.15 0.1099 0.5 60] Base Movement
  ;;[0.15 0.15 0.15 0.5] planer
  (if (Variables|Default|GetCanGlide)
    (Physics|AddForce :Force "2.000000,2.000000,0.000000")
    (Variables|/Script/Engine.CharacterMovementComponent|SetGravityScale _charactermovement_3 0.3)
    (Variables|/Script/Engine.CharacterMovementComponent|SetAirControl _charactermovement_3 0.6)
    (bind _returnvalue (Audio|SpawnSoundatLocation "/Game/Spirit/Blueprints/Son/Cue/WindCue.WindCue" (Transformation|GetActorLocation) "0, 0, 0" 0.7 1.0 0.0 0 0))
    (Class|LegacyCameraShake|StartLegacyCameraShake (Game|GetPlayerCameraManager 0) "/Game/Spirit/Blueprints/Feedbacks/CamShake/BP_FOVGlide.BP_FOVGlide_C" 5.0 "CameraLocal" "0, 0, 0")
    (Utilities|FlowControl|RetriggerableDelay 0.2)
    (CallFunction|UseRessource)
    (CallFunction|RessourceCalc)
    (if (== (Variables|float|GetRessource%20) 0.0)
      (Variables|/Script/Engine.CharacterMovementComponent|SetGravityScale _charactermovement_2 1.0)
      (Variables|/Script/Engine.CharacterMovementComponent|SetAirControl _charactermovement_2 0.05))
    (else
      (Variables|Default|SetJumpMaxCount 1)
      (Variables|/Script/Engine.CharacterMovementComponent|SetGravityScale _charactermovement 1.0)
      (Variables|/Script/Engine.CharacterMovementComponent|SetAirControl _charactermovement 0.05))))

(event Custom|Dash
  (bind _returnvalue (Transformation|GetVelocity))
  (Utilities|FlowControl|Sequence
    (:then_0
      (Utilities|FlowControl|DoOnce false :!label _label
        (:Completed
          (CallFunction|CamShake)
          (if (Variables|Bool|GetIsJumping)
            (Character|LaunchCharacter (* (Class|KismetMathLibrary|VectorNormal2D (Transformation|GetVelocity) 0.0001) (Variables|Default|GetDashStrenghtJump)) false false)
            (Audio|PlaySound2D "/Game/Spirit/Son/musicholder-woosh-260275_cuqYPZ5s.musicholder-woosh-260275_cuqYPZ5s" 0.5 1.5 0.0 0 0)
            (ForceFeedback|SpawnForceFeedbackAttached "/Game/Spirit/Blueprints/Feedbacks/ForceFeedback/FF_Dash.FF_Dash" (Variables|Character|GetMesh) "None" "0, 0, 0" "0, 0, 0" "KeepRelativeOffset" false false 1.0 0.0 0)
            (else
              (Character|LaunchCharacter (Math|Vector|SelectVector (* (Transformation|GetActorForwardVector) 1.2e+03) (* (Class|KismetMathLibrary|VectorNormal2D _returnvalue 0.0001) (Variables|Default|GetDashStrenght)) (< (Math|Vector|VectorLength _returnvalue) 1.0)) false false)
              (Audio|PlaySound2D "/Game/Spirit/Son/musicholder-woosh-260275_cuqYPZ5s.musicholder-woosh-260275_cuqYPZ5s" 0.5 1.5 0.0 0 0)
              (ForceFeedback|SpawnForceFeedbackAttached "/Game/Spirit/Blueprints/Feedbacks/ForceFeedback/FF_Dash.FF_Dash" (Variables|Character|GetMesh) "None" "0, 0, 0" "0, 0, 0" "KeepRelativeOffset" false false 1.0 0.0 0))))))
    (:then_1
      (Utilities|FlowControl|Delay (Variables|Default|GetDashCD))
      (goto _label Reset))))

(event Custom|StopRegen
  ;[1 0.9934 0.1478 0.3565 60] Ressource
  ;;[0.15 0.15 0.15 0.5] Regen
  (Utilities|Time|ClearandInvalidateTimerbyHandle (stale Custom|regen _returnvalue))
  (Utilities|Time|ClearandInvalidateTimerbyHandle (stale Custom|StartRegenRessource _returnvalue)))

(event Custom|regen
  ;[1 0.9934 0.1478 0.3565 60] Ressource
  ;;[0.15 0.15 0.15 0.5] Regen
  (bind _returnvalue (Utilities|Time|SetTimerbyEvent (delegate Custom|StartRegenRessource) 1.0 true)))

(event Custom|AugmentationRessource
  ;[1 0.9934 0.1478 0.3565 60] Ressource
  ;;[0.15 0.15 0.15 0.5] augmentation ressource
  (if (Variables|Bool|GetISRessourceAugmented)
    (Variables|float|SetMaxRessource (+ (Variables|float|GetMaxRessource) 1e+01))
    (Variables|float|SetRessource%20 (+ (Variables|float|GetMaxRessource) 1e+01))))

(event Custom|StopSwimming
  ;[0.15 0 0 0.5 33] Useless
  ;;[0.15 0 0 0.5] Swimm
  (Transformation|AddLocalOffset (Variables|Default|GetCamera) (Math|Vector|MakeVector 0.0 0.0 -12.0) true false)
  (Variables|Bool|SetIsSwimming false))

(event Custom|Swimming
  ;[0.15 0 0 0.5 33] Useless
  ;;[0.15 0 0 0.5] Swimm
  (Variables|Bool|SetIsSwimming (AI|Components|NavMovement|IsSwimming (Variables|Character|GetCharacterMovement) :!class /Script/Engine.NavMovementInterface))
  (Variables|Bool|SetIsSwimming true)
  (Transformation|AddLocalOffset (Variables|Default|GetCamera) "0.000000,0.000000,12.000000" true false))

(event Custom|UseRessource
  ;[0.15 0.15 0.15 0.5] LoseRessource
  (if (Variables|Default|GetIsDash)
    (Variables|float|SetRessource%20 (Math|Float|Clamp(Float) (- (Variables|float|GetRessource%20) 1e+01) 0.0 (Variables|float|GetMaxRessource)))
    (else
      (Variables|float|SetRessource%20 (Math|Float|Clamp(Float) (- (Variables|float|GetRessource%20) 5.0) 0.0 (Variables|float|GetMaxRessource)))))
  (Utilities|FlowControl|RetriggerableDelay 0.2)
  (if (== (Variables|float|GetRessource%20) 0.0)
    (CallFunction|StopSP)
    (CallFunction|RessourceCalc)
    (CallFunction|RessourceCalc)
    (Character|StopJumping)
    (CallFunction|RessourceCalc)
    (Audio|PlaySound2D "/Game/Spirit/Blueprints/Dialogues/Voice/Cue/EnduranceCue/Endurance_Cue.Endurance_Cue" 1.0 1.0 0.0 0 0)
    (else
      (CallFunction|RessourceCalc))))

(event Custom|CamShake
  (Class|LegacyCameraShake|StartLegacyCameraShake (Game|GetPlayerCameraManager 0) "/Game/Spirit/Blueprints/Feedbacks/CamShake/BP_FOV.BP_FOV_C" 1.0 "CameraLocal" "0, 0, 0"))

(event Custom|Respawn
  ;[0.044 0.15 0.1099 0.5 60] Base Movement
  ;;[0.15 0.15 0.15 0.5] Respawn
  (bind _asbpgm_spirit (Utilities|Casting|CastToBPGM_Spirit (Game|GetGameMode)))
  (Transformation|SetActorLocationAndRotation (Variables|/Game/Spirit/Blueprints/Manager/BPGM_Spirit.BPGM_Spirit_C|GetActor%20Location _asbpgm_spirit) (Variables|/Game/Spirit/Blueprints/Manager/BPGM_Spirit.BPGM_Spirit_C|GetActor%20Rotation _asbpgm_spirit) false true))

(event Custom|StartRegenRessource
  ;[1 0.9934 0.1478 0.3565 60] Ressource
  ;;[0.15 0.15 0.15 0.5] Regen
  (bind _returnvalue (Utilities|Time|SetTimerbyEvent (delegate Custom|RegenRessource) 0.1)))

(event Custom|RegenRessource
  ;[1 0.9934 0.1478 0.3565 60] Ressource
  ;;[0.15 0.15 0.15 0.5] Regen
  (Variables|float|SetRessource%20 (Math|Float|Clamp(Float) (+ (Variables|float|GetRessource%20) 15.0) 0.0 (Variables|float|GetMaxRessource)))
  (if (== (Math|Float|Clamp(Float) (+ (Variables|float|GetRessource%20) 15.0) 0.0 (Variables|float|GetMaxRessource)) (Variables|float|GetMaxRessource))
    (CallFunction|StopRegen)))

(event Input|EnhancedActionEvents|EnhancedInputActionIA_Move
  (params (ActionValue :type Vector%202D%20Structure) (ElapsedSeconds :type Float%20%28double-precision%29) (TriggeredSeconds :type Float%20%28double-precision%29) (InputAction :type Input%20Action%20Object%20Reference :default "/Game/Spirit/Inputs/Input_Actions/Fait/IA_Move.IA_Move"))
  (bind _returnvalue (Pawn|GetControlRotation :!class /Script/Engine.Pawn))
  (bind _returnvalue_2 (Pawn|GetControlRotation :!class /Script/Engine.Pawn))
  ;[0.044 0.15 0.1099 0.5 60] Base Movement
  ;;[0.15 0.15 0.15 0.5] base movement
  (:Triggered
    (Variables|Bool|SetIsWalking true)
    (Class|LegacyCameraShake|StartLegacyCameraShake 0 "/Game/Spirit/Blueprints/Feedbacks/CamShake/BP_CamShakeWalk.BP_CamShakeWalk_C" 5.0 "CameraLocal" "0, 0, 0")
    (bind _returnvalue_3 (Audio|SpawnSound2D "/Game/Spirit/Blueprints/Son/Cue/Walk.Walk" 1.0 1.0 0.0 0))
    (if (Variables|Bool|GetIsJumping)
      (Audio|Components|Audio|Stop _returnvalue_3))
    (Utilities|FlowControl|Sequence
      (:then_0
        (if (Variables|Bool|GetIsSwimming)
          (Pawn|Input|AddMovementInput (Math|Vector|GetUpVector _returnvalue) (.y ActionValue) false)
          (Transformation|SetActorRotation _returnvalue)
          (else
            (Pawn|Input|AddMovementInput (Math|Vector|GetRightVector (Math|Rotator|MakeRotator 0.0 0.0 (.yaw (Pawn|GetControlRotation :!class /Script/Engine.Pawn)))) (.x ActionValue) false :!label _label)
            (Pawn|Input|AddMovementInput (Math|Vector|GetForwardVector (Math|Rotator|MakeRotator (.roll _returnvalue_2) 0.0 (.yaw _returnvalue_2))) (.y ActionValue) false))))
      (:then_1
        (goto _label))))
  (:Canceled
    (Variables|Bool|SetIsWalking false :!label _label_2))
  (:Completed
    (goto _label_2)))

(event Input|EnhancedActionEvents|EnhancedInputActionIA_Jump
  (params (ActionValue :type Boolean) (ElapsedSeconds :type Float%20%28double-precision%29) (TriggeredSeconds :type Float%20%28double-precision%29) (InputAction :type Input%20Action%20Object%20Reference :default "/Game/Spirit/Inputs/Input_Actions/Fait/IA_Jump.IA_Jump"))
  ;[0.15 0.15 0.15 0.5] jump && planer
  (:Triggered
    (Variables|Bool|SetIsJumping true)
    (if (Variables|Bool|GetIsGrabbing)
      (Character|StopJumping)
      (else
        (Character|Jump)
        (CallFunction|RessourceCalc)
        (Variables|/Script/Engine.CharacterMovementComponent|SetbNotifyApex (Variables|Character|GetCharacterMovement) true)
        (CallFunction|OnApexReached)
        (Class|LegacyCameraShake|StartLegacyCameraShake (Game|GetPlayerCameraManager 0) "/Game/Spirit/Blueprints/Feedbacks/CamShake/BP_FOVGlide.BP_FOVGlide_C" 1.0 "CameraLocal" "0, 0, 0")
        (Class|LegacyCameraShake|StartLegacyCameraShake (Game|GetPlayerCameraManager 0) "/Game/Spirit/Blueprints/Feedbacks/CamShake/BP_GlideShake.BP_GlideShake_C" 1.0 "CameraLocal" "0, 0, 0")
        (EventDispatchers|UnbindEventfromOnReachedJumpApex (EventDispatchers|CreateEvent :!event Custom|OnApexReached))
        (CallFunction|RessourceCalc)
        (CallFunction|UseRessource))))
  (:Completed
    (Character|StopJumping)
    (Variables|/Script/Engine.CharacterMovementComponent|SetbNotifyApex (Variables|Character|GetCharacterMovement) false)
    (EventDispatchers|UnbindallEventsfromOnReachedJumpApex)
    (Variables|/Script/Engine.CharacterMovementComponent|SetGravityScale (Variables|Character|GetCharacterMovement) 1.0)))

(event Input|EnhancedActionEvents|EnhancedInputActionIA_Pause
  (params (ActionValue :type Boolean) (ElapsedSeconds :type Float%20%28double-precision%29) (TriggeredSeconds :type Float%20%28double-precision%29) (InputAction :type Input%20Action%20Object%20Reference :default "/Game/Spirit/Inputs/Input_Actions/IA_Pause.IA_Pause"))
  (bind _returnvalue (Game|GetPlayerController 0))
  ;[0.15 0.12 0.1312] UI
  ;;[0.15 0.15 0.15 0.5] Pause
  (:Started
    (if (not (Variables|Bool|GetIA_pauseMenuOpen))
      (Variables|Bool|SetIA_pauseMenuOpen true)
      (bind _returnvalue_2 (UserInterface|CreateWidget "/Game/Spirit/Blueprints/Menu/Pause/BPW_Pause.BPW_Pause_C" _returnvalue))
      (bind _output_get (Variables|Default|SetPause%20Menu%20Widget _returnvalue_2))
      (UserInterface|Viewport|AddtoViewport _output_get 0)
      (Input|SetInputModeGameandUI _returnvalue (Variables|Default|GetPause%20Menu%20Widget) "DoNotLock" true false)
      (Variables|/Script/Engine.PlayerController|SetbShowMouseCursor (Game|GetPlayerController 0) true)
      (Utilities|Time|SetGlobalTimeDilation 0.0)))
  (:Canceled
    (Variables|Bool|SetIA_pauseMenuOpen false :!label _label))
  (:Completed
    (goto _label)))

(event Input|EnhancedActionEvents|EnhancedInputActionIA_Look
  (params (ActionValue :type Vector%202D%20Structure) (ElapsedSeconds :type Float%20%28double-precision%29) (TriggeredSeconds :type Float%20%28double-precision%29) (InputAction :type Input%20Action%20Object%20Reference :default "/Game/Spirit/Inputs/Input_Actions/Fait/IA_Look.IA_Look"))
  ;[0.044 0.15 0.1099 0.5 60] Base Movement
  ;;[0.15 0.15 0.15 0.5] look
  (CallFunction|Look (.x ActionValue) (.y ActionValue) 0.0))

(event Input|EnhancedActionEvents|EnhancedInputActionIA_MouseLook
  (params (ActionValue :type Vector :default "0, 0, 0") (ElapsedSeconds :type Float%20%28double-precision%29) (TriggeredSeconds :type Float%20%28double-precision%29) (InputAction :type Input%20Action%20Object%20Reference :default "/Game/Spirit/Inputs/Input_Actions/Fait/IA_MouseLook.IA_MouseLook"))
  ;[0.044 0.15 0.1099 0.5 60] Base Movement
  ;;[0.15 0.15 0.15 0.5] look
  (CallFunction|Look (.x ActionValue) (.y ActionValue) (.z ActionValue)))

(event Input|EnhancedActionEvents|EnhancedInputActionIA_Crouch
  (params (ActionValue :type Boolean) (ElapsedSeconds :type Float%20%28double-precision%29) (TriggeredSeconds :type Float%20%28double-precision%29) (InputAction :type Input%20Action%20Object%20Reference :default "/Game/Spirit/Inputs/Input_Actions/Fait/IA_Crouch.IA_Crouch"))
  ;[0.044 0.15 0.1099 0.5 60] Base Movement
  ;;[0.15 0.15 0.15 0.5] Crouch
  (:Triggered
    (Character|Crouch))
  (:Completed
    (Character|UnCrouch)))

(event Input|EnhancedActionEvents|EnhancedInputActionIA_Interact
  (params (ActionValue :type Boolean) (ElapsedSeconds :type Float%20%28double-precision%29) (TriggeredSeconds :type Float%20%28double-precision%29) (InputAction :type Input%20Action%20Object%20Reference :default "/Game/Spirit/Inputs/Input_Actions/IA_Interact.IA_Interact"))
  ;[0.044 0.15 0.1099 0.5 60] Base Movement
  ;;[0.15 0.15 0.15 0.5] Interactions
  (:Started
    (CallFunction|InteractTrace)
    (bind _lookatactor (Variables|Default|GetLookAtActor)
      (:then
        (bind _objectiveid (Class|BPIInventory|Interact(Message) _lookatactor))
        (Default|CallOnObjectiveIDCalled _objectiveid))
      (:else))))

(event Input|EnhancedActionEvents|EnhancedInputActionIA_Sprint
  (params (ActionValue :type Boolean) (ElapsedSeconds :type Float%20%28double-precision%29) (TriggeredSeconds :type Float%20%28double-precision%29) (InputAction :type Input%20Action%20Object%20Reference :default "/Game/Spirit/Inputs/Input_Actions/Fait/IA_Sprint.IA_Sprint"))
  (bind _returnvalue (Game|GetPlayerCameraManager 0))
  ;[0.044 0.15 0.1099 0.5 60] Base Movement
  ;;[0.15 0.15 0.15 0.5] Sprint
  (:Started
    (if (Variables|Bool|GetSetCanSprint)
      (CallFunction|StartSp)
      (CallFunction|RessourceCalc)
      (Class|LegacyCameraShake|StartLegacyCameraShake _returnvalue "/Game/Spirit/Blueprints/Feedbacks/CamShake/BP_SprintShake.BP_SprintShake_C" 5.0 "CameraLocal" "0, 0, 0")))
  (:Completed
    (CallFunction|StopSP)
    (CallFunction|Regen)
    (Class|PlayerCameraManager|StopAllInstancesOfCameraShake _returnvalue "/Game/Spirit/Blueprints/Feedbacks/CamShake/BP_SprintShake.BP_SprintShake_C" true)))

(event Input|EnhancedActionEvents|EnhancedInputActionIA_Dash
  (params (ActionValue :type Boolean) (ElapsedSeconds :type Float%20%28double-precision%29) (TriggeredSeconds :type Float%20%28double-precision%29) (InputAction :type Input%20Action%20Object%20Reference :default "/Game/Spirit/Inputs/Input_Actions/Fait/IA_Dash.IA_Dash"))
  (if (Variables|Bool|GetCanDash)
    (bind _returnvalue (UserInterface|CreateWidget "/Game/Spirit/Blueprints/Feedbacks/Vignettes/WBP_vignetteDash.WBP_vignetteDash_C" (Game|GetPlayerController 0)))
    (UserInterface|Viewport|AddtoViewport _returnvalue 0)
    (CallFunction|Dash)
    (Variables|Default|SetIsDash true)
    (CallFunction|UseRessource)
    (Widget|RemovefromParent _returnvalue)))

(event Input|EnhancedActionEvents|EnhancedInputActionIA_Grab
  (params (ActionValue :type Boolean) (ElapsedSeconds :type Float%20%28double-precision%29) (TriggeredSeconds :type Float%20%28double-precision%29) (InputAction :type Input%20Action%20Object%20Reference :default "/Game/Spirit/Inputs/Input_Actions/Fait/IA_Grab.IA_Grab"))
  ;[0.15 0 0 0.5 33] Useless
  ;;[0.15 0 0 0.5 30] Grab
)

(event EventBeginPlay
  (bind _returnvalue (Game|GetPlayerController 0))
  (bind _returnvalue_2 (PlayerController|LocalPlayerSubsystems|GetEnhancedInputLocalPlayerSubsystem _returnvalue))
  ;[0.15 0.15 0.15 0.5 50] begin play
  (Input|AddMappingContext _returnvalue_2 "/Game/Spirit/Inputs/IMC_Chara.IMC_Chara" 0 "(bIgnoreAllPressedKeysUntilRelease=True,bForceImmediately=False,bNotifyUserSettings=False)")
  (Input|AddMappingContext _returnvalue_2 "/Game/Spirit/Inputs/IMC_MouseLook.IMC_MouseLook" 0 "(bIgnoreAllPressedKeysUntilRelease=True,bForceImmediately=False,bNotifyUserSettings=False)")
  (bind _output_get (Variables|float|SetMaxRessource 1.5e+02))
  (Variables|float|SetRessource%20 _output_get)
  (Variables|Default|SetMaxHealth 1e+02)
  (Variables|Default|SetCurrentHealth 1e+02)
  (Variables|Bool|SetSetCanSprint true)
  (Variables|Bool|SetCanDash true)
  (Variables|Default|SetCanGlide true)
  (bind _returnvalue_3 (UserInterface|CreateWidget "/Game/Spirit/Blueprints/Menu/WBP_Stamina.WBP_Stamina_C" (Game|GetPlayerController 0)))
  (UserInterface|Viewport|AddtoViewport _returnvalue_3 0))

(event Game|Damage|EventAnyDamage
  (params (Damage :type Float%20%28single-precision%29) (DamageType :type Damage%20Type%20Object%20Reference) (InstigatedBy :type Controller%20Object%20Reference) (DamageCauser :type Actor%20Object%20Reference))
  ;[0.044 0.15 0.1099 0.5 60] Base Movement
  ;;[0.15 0.15 0.15 0.5] TakeDamage
  (bind _output_get (Variables|Default|SetCurrentHealth (Math|Float|Clamp(Float) (- (Variables|Default|GetCurrentHealth) Damage) 0.0 (Variables|Default|GetMaxHealth))))
  (if (== _output_get 0.0)
    _))

(event EventTick
  (params (DeltaSeconds :type Float%20%28single-precision%29))
  ;[0.15 0.15 0.15 0.5 50] tick
  (CallFunction|InteractTrace)
  (if (Variables|Bool|GetIsWalking)
    (Class|LegacyCameraShake|StartLegacyCameraShake (Game|GetPlayerCameraManager 0) "/Game/Spirit/Blueprints/Feedbacks/CamShake/BP_CamShakeWalk.BP_CamShakeWalk_C" 1.0 "CameraLocal" "0, 0, 0")
    (else
      (Class|PlayerCameraManager|StopAllInstancesOfCameraShake (Game|GetPlayerCameraManager 0) "/Game/Spirit/Blueprints/Feedbacks/CamShake/BP_CamShakeWalk.BP_CamShakeWalk_C" true))))

(event EventOnLanded
  (params (Hit :type Hit%20Result%20Structure%20%28by%20ref%29))
  (bind _charactermovement (Variables|Character|GetCharacterMovement))
  ;[0.044 0.15 0.1099 0.5 60] Base Movement
  ;;[0.15 0.15 0.15 0.5] planer
  (Variables|/Script/Engine.CharacterMovementComponent|SetGravityScale _charactermovement 2.0)
  (Variables|/Script/Engine.CharacterMovementComponent|SetAirControl _charactermovement 0.05)
  (Utilities|FlowControl|Delay 0.2)
  (Class|LegacyCameraShake|StartLegacyCameraShake (Game|GetPlayerCameraManager 0) "/Game/Spirit/Blueprints/Feedbacks/CamShake/BP_SprintShake.BP_SprintShake_C" 5.0 "CameraLocal" "0, 0, 0")
  (if (Variables|Bool|GetIsJumping)
    (CallFunction|Regen)
    (Audio|Components|Audio|Stop (stale Custom|OnApexReached _returnvalue))
    (Variables|Bool|SetIsJumping false)))

(event Input|KeyboardEvents|G
  (params (Key :type Key%20Structure :default "None"))
  ;[1 0.9934 0.1478 0.3565 60] Ressource
  ;;[0.15 0.15 0.15 0.5] Regen
  (:Pressed
    (CallFunction|StartRegenRessource)))

(event Input|KeyboardEvents|H
  (params (Key :type Key%20Structure :default "None"))
  ;[0.15 0 0 0.5 33] Useless
  ;;[0.15 0.15 0.15 0.5] Debug
  (:Pressed
    (for _array_element (.Values (Default|GetItems (Variables|Default|GetAC_Inventory)))
      (Development|PrintText (Utilities|Text|FormatText "{name}::{quantity}" (.DisplayName (Utilities|Struct|BreakST_InventoryItem _array_element)) (.Quantity (Utilities|Struct|BreakST_InventoryItem _array_element)))))))

(event Input|KeyboardEvents|G
  (params (Key :type Key%20Structure :default "None"))
  ;[0.044 0.15 0.1099 0.5 60] Base Movement
  (:Pressed
    (CallFunction|Respawn)))

(event Input|KeyboardEvents|J
  (params (Key :type Key%20Structure :default "None"))
  ;[1 0.9934 0.1478 0.3565 60] Ressource
  (:Pressed
    (CallFunction|RegenRessource)))

(fn ConstructionScript)

(fn Look
  (params (Yaw :type Float%20%28double-precision%29) (Pitch :type Float%20%28double-precision%29) (Roll :type Float%20%28double-precision%29))
  (Pawn|Input|AddControllerYawInput Yaw)
  (Pawn|Input|AddControllerPitchInput Pitch)
  (Pawn|Input|AddControllerRollInput Roll))

(fn StartSp
  (Variables|/Script/Engine.CharacterMovementComponent|SetMaxWalkSpeed (Variables|Character|GetCharacterMovement) 7e+02)
  (Variables|Bool|SetIsRunning true)
  (Components|Activation|Activate (Variables|Default|GetNS_Sprint) false))

(fn StopSP
  (Variables|/Script/Engine.CharacterMovementComponent|SetMaxWalkSpeed (Variables|Character|GetCharacterMovement) 4e+02)
  (Variables|Bool|SetIsRunning false)
  (Components|Activation|Deactivate (Variables|Default|GetNS_Sprint)))

(fn RessourceCalc
  (if (Variables|Bool|GetIsRunning)
    (CallFunction|UseRessource)
    (elif (Variables|Bool|GetIsClimbing)
      (CallFunction|UseRessource)
      (elif (Variables|Bool|GetIsGliding)
        (CallFunction|UseRessource)))))

(fn InteractTrace
  (bind _returnvalue (Game|GetPlayerCameraManager 0))
  (bind _returnvalue_2 (Camera|GetCameraLocation _returnvalue))
  (bind (_outhit _returnvalue_3) (Collision|LineTraceByChannel _returnvalue_2 (+ _returnvalue_2 (* (Transformation|GetActorForwardVector _returnvalue) 2e+02)) "TraceTypeQuery2" false 0 "None"))
  (if _returnvalue_3
    (Utilities|IsValid (.HitActor (Collision|BreakHitResult _outhit))
      (:Is%20Valid
        (if (Utilities|DoesObjectImplementInterface (.HitActor (Collision|BreakHitResult _outhit)) "/Game/Spirit/Blueprints/Chara/Inventary/BP/BPI_Inventory.BPI_Inventory_C")
          (bind _output_get (Variables|Default|SetLookAtActor (.HitActor (Collision|BreakHitResult _outhit))))
          (Class|BPIInventory|Lookat(Message) _output_get)
          (else
            (Variables|Default|SetLookAtActor 0)))))
    (else
      (Variables|Default|SetLookAtActor 0))))

(fn Interact
  (return ""))

(fn PickupItem
  (params (ID :type Name :default "None") (DropItem :type ST%20Inventory%20Item%20Structure))
  (Development|PrintString (Utilities|String|ToString(Name) ID))
  (bind _success (Default|Give (Variables|Default|GetAC_Inventory) ID -1 DropItem))
  (return _success))