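; Test player character Blueprint with Enhanced Input movement, jump-apex gliding, swimming, crouching, object grabbing and inventory pickup.
; A resource pool drains during gliding and refills on timers; sprint helpers exist but IA_Sprint is unwired.
; A per-tick camera trace caches BPI_Inventory actors for interaction, while a separate trace attaches "Object"-tagged components for carrying.
; Debug prints and G/H keys expose resource and inventory state.
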(event Custom|OnApexReached
  (bind _charactermovement (Variables|Character|GetCharacterMovement))
  (bind _charactermovement_2 (Variables|Character|GetCharacterMovement))
  ;[0.044 0.15 0.1099 0.5 60] Base Movement
  ;;[0.15 0.15 0.15 0.5] planer
  (Variables|/Script/Engine.CharacterMovementComponent|SetGravityScale _charactermovement_2 0.3)
  (Variables|/Script/Engine.CharacterMovementComponent|SetAirControl _charactermovement_2 0.6)
  (Utilities|FlowControl|RetriggerableDelay 0.2)
  (CallFunction|UseRessource)
  (CallFunction|RessourceCalc)
  (if (== (Variables|float|GetRessource%20) 0.0)
    (Variables|/Script/Engine.CharacterMovementComponent|SetGravityScale _charactermovement 1.0)
    (Variables|/Script/Engine.CharacterMovementComponent|SetAirControl _charactermovement 0.05)))

(event Custom|StopRegen
  ;[1 0.9934 0.1478 0.3565 60] Ressource
  ;;[0.15 0.15 0.15 0.5] Regen
  (Utilities|Time|ClearandInvalidateTimerbyHandle (stale Custom|regen _returnvalue))
  (Utilities|Time|ClearandInvalidateTimerbyHandle (stale Custom|StartRegenRessource _returnvalue)))

(event Custom|regen
  ;[1 0.9934 0.1478 0.3565 60] Ressource
  ;;[0.15 0.15 0.15 0.5] Regen
  (bind _returnvalue (Utilities|Time|SetTimerbyEvent (delegate Custom|StartRegenRessource) 1.0 true)))

(event Custom|AugmentationRessource
  ;[1 0.9934 0.1478 0.3565 60] Ressource
  ;;[0.15 0.15 0.15 0.5] augmentation ressource
  (if (Variables|Bool|GetISRessourceAugmented)
    (bind _output_get (Variables|float|SetMaxRessource (+ (Variables|float|GetMaxRessource) 1e+01)))
    (Variables|float|SetRessource%20 (+ (Variables|float|GetMaxRessource) 1e+01))
    (Development|PrintString (Utilities|String|ToString(Float) _output_get))))

(event Custom|StopSwimming
  ;[0.044 0.15 0.1099 0.5 60] Base Movement
  ;;[0.15 0.15 0.15 0.5] Swimm
  (Transformation|AddLocalOffset (Variables|Default|GetCamera) (Math|Vector|MakeVector 0.0 0.0 -12.0) true false)
  (Variables|Default|SetIsSwimming false))

(event Custom|Swimming
  ;[0.044 0.15 0.1099 0.5 60] Base Movement
  ;;[0.15 0.15 0.15 0.5] Swimm
  (Variables|Default|SetIsSwimming (AI|Components|NavMovement|IsSwimming (Variables|Character|GetCharacterMovement) :!class /Script/Engine.NavMovementInterface))
  (Variables|Default|SetIsSwimming true)
  (Transformation|AddLocalOffset (Variables|Default|GetCamera) "0.000000,0.000000,12.000000" true false))

(event Custom|UseRessource
  ;[1 0.9934 0.1478 0.3565 60] Ressource
  ;;[0.15 0.15 0.15 0.5] LooseRessource
  (Variables|float|SetRessource%20 (Math|Float|Clamp(Float) (- (Variables|float|GetRessource%20) 1e+01) 0.0 (Variables|float|GetMaxRessource)))
  (Development|PrintString (Utilities|String|ToString(Float) (Variables|float|GetRessource%20)))
  (Utilities|FlowControl|RetriggerableDelay 0.2)
  (if (== (Variables|float|GetRessource%20) 0.0)
    (CallFunction|StopSP)
    (CallFunction|RessourceCalc)
    (CallFunction|RessourceCalc)
    (Character|StopJumping)
    (CallFunction|RessourceCalc)
    (else
      (CallFunction|RessourceCalc))))

(event Custom|StartRegenRessource
  ;[1 0.9934 0.1478 0.3565 60] Ressource
  ;;[0.15 0.15 0.15 0.5] Regen
  (bind _returnvalue (Utilities|Time|SetTimerbyEvent (delegate Custom|RegenRessource) 0.2)))

(event Custom|RegenRessource
  ;[1 0.9934 0.1478 0.3565 60] Ressource
  ;;[0.15 0.15 0.15 0.5] Regen
  (Variables|float|SetRessource%20 (Math|Float|Clamp(Float) (+ (Variables|float|GetRessource%20) 1e+04) 0.0 (Variables|float|GetMaxRessource)))
  (if (== (Math|Float|Clamp(Float) (+ (Variables|float|GetRessource%20) 1e+04) 0.0 (Variables|float|GetMaxRessource)) (Variables|float|GetMaxRessource))
    (CallFunction|StopRegen)))

(event Input|EnhancedActionEvents|EnhancedInputActionIA_Move
  (params (ActionValue :type Vector%202D%20Structure) (ElapsedSeconds :type Float%20%28double-precision%29) (TriggeredSeconds :type Float%20%28double-precision%29) (InputAction :type Input%20Action%20Object%20Reference :default "/Game/Spirit/Inputs/Input_Actions/Fait/IA_Move.IA_Move"))
  (bind _returnvalue (Pawn|GetControlRotation :!class /Script/Engine.Pawn))
  (bind _returnvalue_2 (Pawn|GetControlRotation :!class /Script/Engine.Pawn))
  ;[0.044 0.15 0.1099 0.5 60] Base Movement
  ;;[0.15 0.15 0.15 0.5] base movement
  (Utilities|FlowControl|Sequence
    (:then_0
      (if (Variables|Default|GetIsSwimming)
        (Pawn|Input|AddMovementInput (Math|Vector|GetUpVector _returnvalue) (.y ActionValue) false)
        (Transformation|SetActorRotation _returnvalue)
        (else
          (Pawn|Input|AddMovementInput (Math|Vector|GetRightVector (Math|Rotator|MakeRotator 0.0 0.0 (.yaw (Pawn|GetControlRotation :!class /Script/Engine.Pawn)))) (.x ActionValue) false :!label _label)
          (Pawn|Input|AddMovementInput (Math|Vector|GetForwardVector (Math|Rotator|MakeRotator (.roll _returnvalue_2) 0.0 (.yaw _returnvalue_2))) (.y ActionValue) false))))
    (:then_1
      (goto _label))))

(event Input|EnhancedActionEvents|EnhancedInputActionIA_Jump
  (params (ActionValue :type Boolean) (ElapsedSeconds :type Float%20%28double-precision%29) (TriggeredSeconds :type Float%20%28double-precision%29) (InputAction :type Input%20Action%20Object%20Reference :default "/Game/Spirit/Inputs/Input_Actions/Fait/IA_Jump.IA_Jump"))
  ;[0.044 0.15 0.1099 0.5 60] Base Movement
  ;;[0.15 0.15 0.15 0.5] jump && planer
  (:Triggered
    (if (Variables|Bool|GetIsGrabbing)
      (Character|StopJumping)
      (else
        (Character|Jump)
        (CallFunction|RessourceCalc)
        (Variables|/Script/Engine.CharacterMovementComponent|SetbNotifyApex (Variables|Character|GetCharacterMovement) true)
        (CallFunction|OnApexReached)
        (EventDispatchers|UnbindEventfromOnReachedJumpApex (EventDispatchers|CreateEvent :!event Custom|OnApexReached))
        (CallFunction|RessourceCalc))))
  (:Completed
    (Character|StopJumping)
    (Variables|/Script/Engine.CharacterMovementComponent|SetbNotifyApex (Variables|Character|GetCharacterMovement) false)
    (EventDispatchers|UnbindallEventsfromOnReachedJumpApex)
    (Variables|/Script/Engine.CharacterMovementComponent|SetGravityScale (Variables|Character|GetCharacterMovement) 1.0)))

(event Input|EnhancedActionEvents|EnhancedInputActionIA_Look
  (params (ActionValue :type Vector%202D%20Structure) (ElapsedSeconds :type Float%20%28double-precision%29) (TriggeredSeconds :type Float%20%28double-precision%29) (InputAction :type Input%20Action%20Object%20Reference :default "/Game/Spirit/Inputs/Input_Actions/Fait/IA_Look.IA_Look"))
  ;[0.044 0.15 0.1099 0.5 60] Base Movement
  ;;[0.15 0.15 0.15 0.5] look
  (CallFunction|Look (.x ActionValue) (.y ActionValue) 0.0))

(event Input|EnhancedActionEvents|EnhancedInputActionIA_MouseLook
  (params (ActionValue :type Vector :default "0, 0, 0") (ElapsedSeconds :type Float%20%28double-precision%29) (TriggeredSeconds :type Float%20%28double-precision%29) (InputAction :type Input%20Action%20Object%20Reference :default "/Game/Spirit/Inputs/Input_Actions/Fait/IA_MouseLook.IA_MouseLook"))
  ;[0.044 0.15 0.1099 0.5 60] Base Movement
  ;;[0.15 0.15 0.15 0.5] look
  (CallFunction|Look (.x ActionValue) (.y ActionValue) (.z ActionValue)))

(event Input|EnhancedActionEvents|EnhancedInputActionIA_Crouch
  (params (ActionValue :type Boolean) (ElapsedSeconds :type Float%20%28double-precision%29) (TriggeredSeconds :type Float%20%28double-precision%29) (InputAction :type Input%20Action%20Object%20Reference :default "/Game/Spirit/Inputs/Input_Actions/Fait/IA_Crouch.IA_Crouch"))
  ;[0.044 0.15 0.1099 0.5 60] Base Movement
  ;;[0.15 0.15 0.15 0.5] Crouch
  (:Triggered
    (Character|Crouch))
  (:Completed
    (Character|UnCrouch)))

(event Input|EnhancedActionEvents|EnhancedInputActionIA_Interact
  (params (ActionValue :type Boolean) (ElapsedSeconds :type Float%20%28double-precision%29) (TriggeredSeconds :type Float%20%28double-precision%29) (InputAction :type Input%20Action%20Object%20Reference :default "/Game/Spirit/Inputs/Input_Actions/IA_Interact.IA_Interact"))
  ;[0.044 0.15 0.1099 0.5 60] Base Movement
  ;;[0.15 0.15 0.15 0.5] Interactions
  (:Started
    (CallFunction|InteractTrace)
    (bind _lookatactor (Variables|Default|GetLookAtActor)
      (:then
        (bind _objectiveid (Class|BPIInventory|Interact(Message) _lookatactor))
        (Default|CallOnObjectiveIDCalled _objectiveid))
      (:else))))

(event Input|EnhancedActionEvents|EnhancedInputActionIA_Sprint
  (params (ActionValue :type Boolean) (ElapsedSeconds :type Float%20%28double-precision%29) (TriggeredSeconds :type Float%20%28double-precision%29) (InputAction :type Input%20Action%20Object%20Reference :default "/Game/Spirit/Inputs/Input_Actions/Fait/IA_Sprint.IA_Sprint"))
  ;[0.044 0.15 0.1099 0.5 60] Base Movement
  ;;[0.15 0.15 0.15 0.5] Sprint
)

(event Input|EnhancedActionEvents|EnhancedInputActionIA_Grab
  (params (ActionValue :type Boolean) (ElapsedSeconds :type Float%20%28double-precision%29) (TriggeredSeconds :type Float%20%28double-precision%29) (InputAction :type Input%20Action%20Object%20Reference :default "/Game/Spirit/Inputs/Input_Actions/Fait/IA_Grab.IA_Grab"))
  (bind _box (Variables|Default|GetBox))
  (bind _returnvalue (Transformation|GetWorldLocation _box))
  ;[0.044 0.15 0.1099 0.5 60] Base Movement
  ;;[0.15 0.15 0.15 0.5 30] Grab
  (:Triggered
    (bind (_outhit _returnvalue_2) (Collision|LineTraceByChannel _returnvalue (+ _returnvalue (* (Math|Vector|GetForwardVector (Variables|Default|GetCamera)) 3e+02)) "TraceTypeQuery1" false 0 "Persistent"))
    (if _returnvalue_2
      (if (Components|ComponentHasTag (.HitComponent (Collision|BreakHitResult _outhit)) "Object")
        (bind _returnvalue_3 (Transformation|AttachComponentToComponent (.HitComponent (Collision|BreakHitResult _outhit)) (Variables|Default|GetBox) "" "SnapToTarget" "KeepWorld" "KeepWorld" true))
        (Variables|Bool|SetIsGrabbing _returnvalue_3)
        (elif (Components|ComponentHasTag (.HitComponent (Collision|BreakHitResult _outhit)) "Poeme")
          _))))
  (:Completed
    (if (Variables|Bool|GetIsGrabbing)
      (Transformation|DetachFromComponent (.HitComponent (Collision|BreakHitResult _outhit)) "KeepWorld" "KeepRelative" "KeepRelative" false)
      (Variables|Bool|SetIsGrabbing false))))

(event EventBeginPlay
  (bind _returnvalue (Game|GetPlayerController 0))
  (bind _returnvalue_2 (PlayerController|LocalPlayerSubsystems|GetEnhancedInputLocalPlayerSubsystem _returnvalue))
  ;[0.15 0.15 0.15 0.5 50] begin play
  (Input|AddMappingContext _returnvalue_2 "/Game/Spirit/Inputs/IMC_Chara.IMC_Chara" 0 "(bIgnoreAllPressedKeysUntilRelease=True,bForceImmediately=False,bNotifyUserSettings=False)")
  (Input|AddMappingContext _returnvalue_2 "/Game/Spirit/Inputs/IMC_MouseLook.IMC_MouseLook" 0 "(bIgnoreAllPressedKeysUntilRelease=True,bForceImmediately=False,bNotifyUserSettings=False)")
  (Variables|float|SetMaxRessource 1e+04))

(event EventTick
  (params (DeltaSeconds :type Float%20%28single-precision%29))
  ;[0.15 0.15 0.15 0.5 50] tick
  (CallFunction|InteractTrace)
  (Development|PrintString (Utilities|String|ToString(Float) (Variables|/Script/Engine.CharacterMovementComponent|GetMaxWalkSpeed (Variables|Character|GetCharacterMovement)))))

(event EventOnLanded
  (params (Hit :type Hit%20Result%20Structure%20%28by%20ref%29))
  (bind _charactermovement (Variables|Character|GetCharacterMovement))
  ;[0.044 0.15 0.1099 0.5 60] Base Movement
  ;;[0.15 0.15 0.15 0.5] planer
  (Variables|/Script/Engine.CharacterMovementComponent|SetGravityScale _charactermovement 2.0)
  (Variables|/Script/Engine.CharacterMovementComponent|SetAirControl _charactermovement 0.05)
  (Utilities|FlowControl|Delay 0.2)
  (CallFunction|StartRegenRessource)
  (Development|PrintString (Utilities|String|ToString(Float) (Variables|float|GetRessource%20))))

(event Input|KeyboardEvents|G
  (params (Key :type Key%20Structure :default "None"))
  ;[1 0.9934 0.1478 0.3565 60] Ressource
  ;;[0.15 0.15 0.15 0.5] Regen
  (:Pressed
    (CallFunction|StartRegenRessource)
    (Development|PrintString (Utilities|String|ToString(Float) (Variables|float|GetRessource%20)))))

(event Input|KeyboardEvents|H
  (params (Key :type Key%20Structure :default "None"))
  ;[0.15 0.15 0.15 0.5] Debug
  (:Pressed
    (for _array_element (.Values (Default|GetItems (Variables|Default|GetAC_Inventory)))
      (Development|PrintText (Utilities|Text|FormatText "{name}::{quantity}" (.DisplayName (Utilities|Struct|BreakST_InventoryItem _array_element)) (.Quantity (Utilities|Struct|BreakST_InventoryItem _array_element)))))))

(fn ConstructionScript)

(fn Look
  (params (Yaw :type Float%20%28double-precision%29) (Pitch :type Float%20%28double-precision%29) (Roll :type Float%20%28double-precision%29))
  (Pawn|Input|AddControllerYawInput Yaw)
  (Pawn|Input|AddControllerPitchInput Pitch)
  (Pawn|Input|AddControllerRollInput Roll))

(fn StartSp
  (Variables|/Script/Engine.CharacterMovementComponent|SetMaxWalkSpeed (Variables|Character|GetCharacterMovement) 7e+02)
  (Variables|Bool|SetIsRunning true))

(fn StopSP
  (Variables|/Script/Engine.CharacterMovementComponent|SetMaxWalkSpeed (Variables|Character|GetCharacterMovement) 4e+02)
  (Variables|Bool|SetIsRunning false))

(fn RessourceCalc
  (if (Variables|Bool|GetIsRunning)
    (CallFunction|UseRessource)
    (elif (Variables|Bool|GetIsClimbing)
      (CallFunction|UseRessource)
      (elif (Variables|Bool|GetIsGliding)
        (CallFunction|UseRessource)))))

(fn InteractTrace
  (bind _returnvalue (Game|GetPlayerCameraManager 0))
  (bind _returnvalue_2 (Camera|GetCameraLocation _returnvalue))
  (bind (_outhit _returnvalue_3) (Collision|LineTraceByChannel _returnvalue_2 (+ _returnvalue_2 (* (Transformation|GetActorForwardVector _returnvalue) 2e+02)) "TraceTypeQuery2" false 0 "None"))
  (if _returnvalue_3
    (Utilities|IsValid (.HitActor (Collision|BreakHitResult _outhit))
      (:Is%20Valid
        (Development|PrintString (Utilities|GetDisplayName (.HitActor (Collision|BreakHitResult _outhit))))
        (if (Utilities|DoesObjectImplementInterface (.HitActor (Collision|BreakHitResult _outhit)) "/Game/Spirit/Blueprints/Chara/Inventary/BP/BPI_Inventory.BPI_Inventory_C")
          (bind _output_get (Variables|Default|SetLookAtActor (.HitActor (Collision|BreakHitResult _outhit))))
          (Class|BPIInventory|Lookat(Message) _output_get)
          (else
            (Variables|Default|SetLookAtActor 0)))))
    (else
      (Variables|Default|SetLookAtActor 0))))

(fn Interact
  (return ""))

(fn PickupItem
  (params (ID :type Name :default "None") (DropItem :type ST%20Inventory%20Item%20Structure))
  (Development|PrintString (Utilities|String|ToString(Name) ID))
  (bind _success (Default|Give (Variables|Default|GetAC_Inventory) ID -1 DropItem))
  (return _success))