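; Base quest actor that tracks the player's progress on the objectives of the current quest stage.
; On BeginPlay it binds to the player character's objective-ID event and loads its stage from the quest data table, zeroing a progress map keyed by objective ID.
; Matching events add to unfinished objectives.
; Any objective reaching its quantity sets IsCompleted and shows a notification widget; stage advancement is absent here.
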(event EventBeginPlay
  (EventDispatchers|BindEventtoOnObjectiveIDCalled (CallFunction|GetPlayerCharacter) (EventDispatchers|CreateEvent :!event OnObjectiveIDHeard))
  (CallFunction|GetQuestDetails))

(event Collision|EventActorBeginOverlap
  (params (OtherActor :type Actor%20Object%20Reference)))

(event EventTick
  (params (DeltaSeconds :type Float%20%28single-precision%29)))

(fn ConstructionScript)

(fn OnObjectiveIDHeard
  (params (ObjectiveID :type String) (Value :type Integer))
  (bind _currentobjectiveprogress (Variables|Default|GetCurrentObjectiveProgress))
  (bind (_value _returnvalue) (Utilities|Map|Find _currentobjectiveprogress ObjectiveID))
  (if _returnvalue
    (if (< _value (Utilities|Struct|BreakS_ObjectivesDetails (CallFunction|GetObjectiveDatabyID ObjectiveID)))
      (Utilities|Map|Add (Variables|Default|GetCurrentObjectiveProgress) ObjectiveID (+ _value Value))
      (CallFunction|IsObjectiveComplete ObjectiveID)
      (return))
    (else
      (return))))

(fn GetQuestDetails
  (bind _returnvalue (Utilities|GetDataTableRow "/Game/Spirit/Blueprints/Quests/QuestBase/Struct/QuestData.QuestData" (Variables|Default|GetQuestID))
    (:then
      (bind _output_get (Variables|Default|SetF_QuestDetails _returnvalue))
      (bind _output_get_2 (Variables|Default|SetCurrentStageDetails (Utilities|Array|Get(acopy) (Utilities|Struct|BreakS_QuestDetails _output_get) (Variables|Default|GetCurrentStage))))
      (Utilities|Map|Clear (Variables|Default|GetCurrentObjectiveProgress))
      (for _array_element (Utilities|Struct|BreakS_StageDetails _output_get_2)
        (Development|PrintString (Utilities|String|ToString(Integer) (.Quantity (Utilities|Struct|BreakS_ObjectivesDetails _array_element))))
        (Utilities|Map|Add (Variables|Default|GetCurrentObjectiveProgress) (.ObjectiveID (Utilities|Struct|BreakS_ObjectivesDetails _array_element)) 0)
        (Development|PrintString "Hello")))))

(fn IsObjectiveComplete
  (params (ObjectiveID :type String))
  (bind _array_element (CallFunction|GetObjectiveDatabyID ObjectiveID))
  (bind (_name _description _type _objectiveid _quantity) (Utilities|Struct|BreakS_ObjectivesDetails _array_element))
  (if (>= (.Value (Utilities|Map|Find (Variables|Default|GetCurrentObjectiveProgress) ObjectiveID)) _quantity)
    (Variables|Default|SetIsCompleted true)
    (bind _returnvalue (UserInterface|CreateWidget "/Game/Spirit/UI/UI_Quest/Quests/WBP_QuestNotification.WBP_QuestNotification_C" 0 _description))
    (UserInterface|Viewport|AddtoViewport _returnvalue 0)))

(fn GetObjectiveDatabyID
  (params (ObjectiveID :type String))
  (for _array_element (.Objectives (Utilities|Struct|BreakS_StageDetails (Variables|Default|GetCurrentStageDetails)))
    (if (Utilities|Enum|Equal(Enum) (Utilities|Struct|BreakS_ObjectivesDetails _array_element) ObjectiveID)
      (return _array_element))))