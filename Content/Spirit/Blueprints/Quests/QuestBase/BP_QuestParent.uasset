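; Base quest character that caches the player and game mode, then starts behavior chosen by its quest enum.
; The Mountain quest swaps in a mannequin mesh, sets walk speed and runs a looping timer that AI-moves it toward the player, turning to face them.
; A fishing (Peche) quest is stubbed with an empty initialization event.
; Ending the quest shows a test UI widget and destroys the actor.
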(event Custom|Initialisation%20Enemy
  (switch Utilities|FlowControl|Switch|SwitchonE_QuestType (Variables|Default|GetQuestEnum)
    (:NewEnumerator3
      (CallFunction|FollowSoulStart))))

(event Custom|FollowSoul_Start
  ;[0.15 0.15 0.15 0.5] Quest Mountain
  (bind _returnvalue (Utilities|Time|SetTimerbyEvent (delegate Custom|Follow) 0.25 true))
  (Variables|Default|SetTimerHandle _returnvalue)
  (Variables|/Script/Engine.CharacterMovementComponent|SetMaxWalkSpeed (Variables|Character|GetCharacterMovement) 4e+02)
  (Components|SkeletalMesh|SetSkeletalMeshAsset (Variables|Character|GetMesh) "/Game/Characters/Mannequins/Meshes/SKM_Manny_Simple.SKM_Manny_Simple"))

(event Custom|Follow
  ;[0.15 0.15 0.15 0.5] Quest Mountain
  (AI|AIMoveTo self "0, 0, 0" (Variables|Default|GetPlayer) 5.0 false
    (:then
      (Transformation|SetActorRotation self (Math|Rotator|MakeRotator 0.0 0.0 (.yaw (Math|Rotator|FindLookatRotation (Transformation|GetActorLocation self) (Transformation|GetActorLocation (Variables|Default|GetPlayer)))))))))

(event Custom|EndQuest
  (bind _returnvalue (UserInterface|CreateWidget "/Game/Spirit/UI/UI_Quest/UI_Test.UI_Test_C"))
  (UserInterface|Viewport|AddtoViewport _returnvalue 0)
  (Actor|DestroyActor))

(event Custom|Quest_Peche
  (bind _returnvalue (Utilities|Time|SetTimerbyEvent (delegate Custom|Initialisation_Peche) 0.0))
  (Variables|Default|SetTimerHandle _returnvalue)
  (Components|SkeletalMesh|SetSkeletalMeshAsset (Variables|Character|GetMesh) "/Game/Characters/Mannequins/Meshes/SKM_Manny_Simple.SKM_Manny_Simple"))

(event Custom|Initialisation_Peche)

(event EventBeginPlay
  (bind _returnvalue (Actor|GetActorOfClass "/Game/Spirit/Blueprints/Chara/BP_Chara.BP_Chara_C"))
  (Variables|Default|SetPlayer _returnvalue)
  (bind _returnvalue_2 (Actor|GetActorOfClass "/Game/Spirit/Blueprints/Manager/BPGM_Spirit.BPGM_Spirit_C"))
  (Variables|Default|SetGame%20Manager _returnvalue_2))

(event Collision|EventActorBeginOverlap
  (params (OtherActor :type Actor%20Object%20Reference)))

(event EventTick
  (params (DeltaSeconds :type Float%20%28single-precision%29)))

(fn ConstructionScript)