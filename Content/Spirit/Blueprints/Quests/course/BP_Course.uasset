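; Timed car race quest that moves the player from their character into a car for the length of GameTimer.
; StartEvent spawns a BP_Cars at each StartPosition, possesses a random one, swaps the input mapping to IMC_Cars and stores the other cars' count in DestroyCars.
; When the timer fires, Leave re-possesses the Character, restores IMC_Chara and destroys every BP_Cars in the world.
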(event Custom|LeaveCars
  (CallFunction|Leave))

(event EventStartEvent
  (params (Chara :type BP%20Chara%20Object%20Reference))
  (bind _returnvalue (Game|GetPlayerController 0))
  (bind _returnvalue_2 (PlayerController|LocalPlayerSubsystems|GetEnhancedInputLocalPlayerSubsystem _returnvalue))
  (CallFunction|StartEvent Chara)
  (for _array_element (Variables|Default|GetStartPosition)
    (Game|SpawnActorfromClass "/Game/Spirit/Blueprints/Quests/course/BP_Cars.BP_Cars_C" (Math|Transform|MakeTransform (Transformation|GetActorLocation _array_element) "0, 0, 0" "1.000000,1.000000,1.000000") "Undefined" "MultiplyWithRoot" 0 0))
  (bind _outactors (Actor|GetAllActorsOfClass "/Game/Spirit/Blueprints/Quests/course/BP_Cars.BP_Cars_C"))
  (bind _output_get (Variables|Default|SetDestroyCars (Utilities|Array|Length _outactors)))
  (Math|Integer|DecrementInt _output_get
    (:%20%20
      (Pawn|Possess (Game|GetPlayerController 0) (.OutItem (Utilities|Array|Random _outactors)))
      (Input|RemoveMappingContext _returnvalue_2 "/Game/Spirit/Inputs/IMC_Chara.IMC_Chara" "(bIgnoreAllPressedKeysUntilRelease=True,bForceImmediately=False,bNotifyUserSettings=False)")
      (Input|AddMappingContext _returnvalue_2 "/Game/Spirit/Blueprints/Quests/course/IMC_Cars.IMC_Cars" 0 "(bIgnoreAllPressedKeysUntilRelease=True,bForceImmediately=False,bNotifyUserSettings=False)")
      (Variables|Default|SetIsPlaying true)
      (Utilities|Time|SetTimerbyEvent (delegate Custom|LeaveCars) (Variables|Default|Getgame%20timer)))))

(fn ConstructionScript
  (|CallParentFunction))

(fn Leave
  (bind _returnvalue (Game|GetPlayerController 0))
  (bind _returnvalue_2 (PlayerController|LocalPlayerSubsystems|GetEnhancedInputLocalPlayerSubsystem _returnvalue))
  (Pawn|UnPossess _returnvalue)
  (Pawn|Possess _returnvalue (Variables|Default|GetCharacter))
  (Input|RemoveMappingContext _returnvalue_2 "/Game/Spirit/Blueprints/Quests/course/IMC_Cars.IMC_Cars" "(bIgnoreAllPressedKeysUntilRelease=True,bForceImmediately=False,bNotifyUserSettings=False)")
  (Input|AddMappingContext _returnvalue_2 "/Game/Spirit/Inputs/IMC_Chara.IMC_Chara" 0 "(bIgnoreAllPressedKeysUntilRelease=True,bForceImmediately=False,bNotifyUserSettings=False)")
  (bind _outactors (Actor|GetAllActorsOfClass "/Game/Spirit/Blueprints/Quests/course/BP_Cars.BP_Cars_C"))
  (for _array_element _outactors
    (Actor|DestroyActor _array_element)))

(fn StopPlaying
  (|CallParentFunction))