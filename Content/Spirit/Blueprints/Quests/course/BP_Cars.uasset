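; BP_Cars is an input-driven physics car whose Car component is moved by force and turned by direct rotation.
; Move input pushes along the forward vector only while Onground is set; turn input applies world roll, not yaw, at any time.
; Onground is set by hits against other BP_Cars actors only and cleared every Tick.
; BeginPlay sends a random unit vector to the materials, though the parameter name is None.
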(event OnComponentHit(car)
  (params (HitComponent :type Primitive%20Component%20Object%20Reference) (OtherActor :type Actor%20Object%20Reference) (OtherComp :type Primitive%20Component%20Object%20Reference) (NormalImpulse :type Vector :default "0, 0, 0") (Hit :type Hit%20Result%20Structure%20%28by%20ref%29))
  (Utilities|Casting|CastToBP_Cars OtherActor)
  (Variables|Default|SetOnground true))

(event Input|EnhancedActionEvents|EnhancedInputActionIA_Move_BP_Car
  (params (ActionValue :type Float%20%28double-precision%29) (ElapsedSeconds :type Float%20%28double-precision%29) (TriggeredSeconds :type Float%20%28double-precision%29) (InputAction :type Input%20Action%20Object%20Reference :default "/Game/Spirit/Blueprints/Quests/course/IA_Move_BP_Car.IA_Move_BP_Car"))
  (bind _car (Variables|Default|Getcar))
  (if (Variables|Default|GetOnground)
    (Physics|AddForce _car (* (* ActionValue (Variables|Default|Getmove%20force)) (Math|Vector|GetForwardVector _car)) "None" false)))

(event Input|EnhancedActionEvents|EnhancedInputActionIA_Turn_BP_Car
  (params (ActionValue :type Float%20%28double-precision%29) (ElapsedSeconds :type Float%20%28double-precision%29) (TriggeredSeconds :type Float%20%28double-precision%29) (InputAction :type Input%20Action%20Object%20Reference :default "/Game/Spirit/Blueprints/Quests/course/IA_Turn_BP_Car.IA_Turn_BP_Car"))
  (Transformation|AddWorldRotation (Variables|Default|Getcar) (Math|Rotator|MakeRotator (* ActionValue (Variables|Default|GetRotation%20Force)) 0.0 0.0) false false))

(event EventBeginPlay
  (Rendering|Material|SetVectorParameterValueonMaterials (Variables|Default|Getcar) "None" (Math|Random|RandomUnitVector)))

(event EventTick
  (params (DeltaSeconds :type Float%20%28single-precision%29))
  (Variables|Default|SetOnground false))

(fn ConstructionScript)