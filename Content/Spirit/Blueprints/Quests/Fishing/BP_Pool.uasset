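; BP_Pool is a fishing pool that starts a quick-time event when its trigger box is overlapped.
; The overlap shows WBP_QTE, disables player movement and switches to cursor-driven Game and UI input.
; SpawnFish removes a valid widget, spawns a BP_Fish of random type at the pool, then restores walking and game-only input.
; FailQTE only removes the widget, without restoring movement or input.
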(event OnComponentBeginOverlap(triggerbox)
  (params (OverlappedComponent :type Primitive%20Component%20Object%20Reference) (OtherActor :type Actor%20Object%20Reference) (OtherComp :type Primitive%20Component%20Object%20Reference) (OtherBodyIndex :type Integer) (bFromSweep :type Boolean) (SweepResult :type Hit%20Result%20Structure%20%28by%20ref%29))
  (bind _returnvalue (Game|GetPlayerController 0))
  ;[0.15 0.15 0.15 0.5] trigger
  (bind _returnvalue_2 (UserInterface|CreateWidget "/Game/Spirit/UI/UI_Quest/WBP_QTE.WBP_QTE_C"))
  (bind _output_get (Variables|Default|SetQTE_Widget _returnvalue_2))
  (UserInterface|Viewport|AddtoViewport _output_get 0)
  (Input|ResetIgnoreLookInput _returnvalue)
  (Variables|/Script/Engine.PlayerController|SetbShowMouseCursor _returnvalue true)
  (Input|SetInputModeGameandUI (Game|GetPlayerController 0) 0 "DoNotLock" true false)
  (Pawn|Components|CharacterMovement|DisableMovement (Variables|/Script/Engine.Character|GetCharacterMovement (Game|GetPlayerCharacter 0))))

(event Custom|SpawnFish
  (bind _returnvalue (Game|GetPlayerController 0))
  ;[0.15 0.15 0.15 0.5] Spawn
  (Utilities|FlowControl|Sequence
    (:then_0
      (bind _qte_widget (Variables|Default|GetQTE_Widget)
        (:then
          (Widget|RemovefromParent _qte_widget)
          (Variables|Default|SetQTE_Widget 0)
          (Development|PrintString "ok")
          (Game|SpawnActorfromClass "/Game/Spirit/Blueprints/Quests/Fishing/BP_Fish.BP_Fish_C" (Transformation|GetActorTransform) "AdjustIfPossibleButAlwaysSpawn" "MultiplyWithRoot" 0 (.OutItem (Utilities|Array|Random (Variables|Default|GetFishEnum))) 0)
          (Variables|Default|SetHasSpawned true))
        (:else)))
    (:then_1
      (Input|ResetIgnoreLookInput _returnvalue)
      (Variables|/Script/Engine.PlayerController|SetbShowMouseCursor _returnvalue false)
      (Input|SetInputModeGameOnly _returnvalue false)
      (Pawn|Components|CharacterMovement|SetMovementMode (Variables|/Script/Engine.Character|GetCharacterMovement (Game|GetPlayerCharacter 0)) "MOVE_Walking" 0)
      (if (Variables|Default|GetHasSpawned)
        (Widget|RemovefromParent (Variables|Default|GetQTE_Widget))))))

(event Custom|FailQTE
  (Widget|RemovefromParent (Variables|Default|GetQTE_Widget)))

(event EventBeginPlay)

(event Collision|EventActorBeginOverlap
  (params (OtherActor :type Actor%20Object%20Reference)))

(event EventTick
  (params (DeltaSeconds :type Float%20%28single-precision%29)))

(fn ConstructionScript)