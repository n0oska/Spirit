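; BPGM_Spirit is a manager Blueprint, apparently the Spirit game mode, with the beginnings of a character respawn system.
; On BeginPlay it finds and caches the BP_Chara character and the BP_Respawn actor.
; Its respawn event only branches on the character's IsDead flag with no action, and the nodes reading the respawn point's location and rotation are left unconnected.
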(event Custom|respawn
  (if (Variables|/Game/Spirit/Blueprints/Chara/BP_Chara.BP_Chara_C|GetIsDead (Variables|Default|GetBp_Chara))
    _))

(event EventBeginPlay
  (bind _returnvalue (Actor|GetActorOfClass "/Game/Spirit/Blueprints/Chara/BP_Chara.BP_Chara_C"))
  (Variables|Default|SetBp_Chara _returnvalue)
  (bind _returnvalue_2 (Actor|GetActorOfClass "/Game/Spirit/Blueprints/Enviro/BP_Respawn.BP_Respawn_C"))
  (Variables|Default|SetBP_respawn _returnvalue_2))

(event EventTick
  (params (DeltaSeconds :type Float%20%28single-precision%29)))

(fn ConstructionScript)