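; BP_SpawnerManager is a one-shot trigger spawner that creates an enemy when the player character (BP_Chara) enters its box.
; The box overlap calls Spawn, which places a BP_IAParent at the manager's own transform, adjusting for collisions but always spawning.
; It assigns the enemy a fixed QuestEnum value, calls InitialisationEnemy, then sets Spawned to block repeat spawns.
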(event OnComponentBeginOverlap(Box)
  (params (OverlappedComponent :type Primitive%20Component%20Object%20Reference) (OtherActor :type Actor%20Object%20Reference) (OtherComp :type Primitive%20Component%20Object%20Reference) (OtherBodyIndex :type Integer) (bFromSweep :type Boolean) (SweepResult :type Hit%20Result%20Structure%20%28by%20ref%29))
  (Utilities|Casting|CastToBP_Chara OtherActor)
  (if (not (Variables|Default|GetSpawned))
    (CallFunction|Spawn)))

(event Custom|Spawn
  (bind _returnvalue (Game|SpawnActorfromClass "/Game/Spirit/Blueprints/Quests/QuestBase/BP_IAParent.BP_IAParent_C" (Transformation|GetActorTransform self) "AdjustIfPossibleButAlwaysSpawn" "MultiplyWithRoot" 0 0))
  (Variables|/Game/Spirit/Blueprints/Quests/QuestBase/BP_IAParent.BP_IAParent_C|SetQuestEnum _returnvalue "NewEnumerator3")
  (Default|InitialisationEnemy _returnvalue)
  (Variables|Default|SetSpawned true))

(event EventBeginPlay)

(event Collision|EventActorBeginOverlap
  (params (OtherActor :type Actor%20Object%20Reference)))

(event EventTick
  (params (DeltaSeconds :type Float%20%28single-precision%29)))

(fn ConstructionScript)