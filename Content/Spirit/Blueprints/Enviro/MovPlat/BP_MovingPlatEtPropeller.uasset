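; Moving platform with a propeller that lifts the player character and quest characters who enter its volume.
; The construction script sets InterpToMovement to travel between two relative points, Loc1 and Loc2, over a configurable Duration.
; Overlapping PropellerColl inverts gravity scale on BP_Chara or BP_QuestParent, sets a small upward velocity and adds a downward force.
; Leaving the volume restores gravity scale to normal.
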(event OnComponentBeginOverlap(PropellerColl)
  (params (OverlappedComponent :type Primitive%20Component%20Object%20Reference) (OtherActor :type Actor%20Object%20Reference) (OtherComp :type Primitive%20Component%20Object%20Reference) (OtherBodyIndex :type Integer) (bFromSweep :type Boolean) (SweepResult :type Hit%20Result%20Structure%20%28by%20ref%29))
  (Utilities|FlowControl|Sequence
    (:then_0
      (bind _asbp_chara (Utilities|Casting|CastToBP_Chara OtherActor))
      (Variables|/Script/Engine.CharacterMovementComponent|SetGravityScale (Variables|/Script/Engine.Character|GetCharacterMovement _asbp_chara) -1.0)
      (Variables|/Script/Engine.MovementComponent|SetVelocity (Variables|/Script/Engine.Character|GetCharacterMovement _asbp_chara) "0.000000,0.000000,30.000000")
      (Physics|AddForce (Variables|/Script/Engine.Character|GetCharacterMovement _asbp_chara) "0.000000,0.000000,-100.000000"))
    (:then_1
      (bind _asbp_quest_parent (Utilities|Casting|CastToBP_QuestParent OtherActor))
      (Variables|/Script/Engine.CharacterMovementComponent|SetGravityScale (Variables|/Script/Engine.Character|GetCharacterMovement _asbp_quest_parent) -1.0)
      (Variables|/Script/Engine.MovementComponent|SetVelocity (Variables|/Script/Engine.Character|GetCharacterMovement _asbp_quest_parent) "0.000000,0.000000,30.000000")
      (Physics|AddForce (Variables|/Script/Engine.Character|GetCharacterMovement _asbp_quest_parent) "0.000000,0.000000,-100.000000"))))

(event OnComponentEndOverlap(PropellerColl)
  (params (OverlappedComponent :type Primitive%20Component%20Object%20Reference) (OtherActor :type Actor%20Object%20Reference) (OtherComp :type Primitive%20Component%20Object%20Reference) (OtherBodyIndex :type Integer))
  (Utilities|FlowControl|Sequence
    (:then_0
      (bind _asbp_chara (Utilities|Casting|CastToBP_Chara OtherActor))
      (Variables|/Script/Engine.CharacterMovementComponent|SetGravityScale (Variables|/Script/Engine.Character|GetCharacterMovement _asbp_chara) 1.0))
    (:then_1
      (bind _asbp_quest_parent (Utilities|Casting|CastToBP_QuestParent OtherActor))
      (Variables|/Script/Engine.CharacterMovementComponent|SetGravityScale (Variables|/Script/Engine.Character|GetCharacterMovement _asbp_quest_parent) 1.0))))

(event EventBeginPlay)

(event Collision|EventActorBeginOverlap
  (params (OtherActor :type Actor%20Object%20Reference)))

(event EventTick
  (params (DeltaSeconds :type Float%20%28single-precision%29)))

(fn ConstructionScript
  (bind _interptomovement (Variables|Default|GetInterpToMovement))
  (Variables|/Script/Engine.InterpToMovementComponent|SetControlPoints _interptomovement (Utilities|Array|MakeArray (Utilities|Struct|MakeInterpControlPoint (Variables|Default|GetLoc1) true) (Utilities|Struct|MakeInterpControlPoint (Variables|Default|GetLoc2) true)))
  (Variables|/Script/Engine.InterpToMovementComponent|SetDuration _interptomovement (Variables|Default|GetDuration)))