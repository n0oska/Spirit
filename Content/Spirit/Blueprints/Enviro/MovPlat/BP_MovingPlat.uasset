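; Moving rock platform actor that travels between two designer-set relative points, Loc1 and Loc2.
; The construction script feeds both points and the Duration variable into an InterpToMovement component.
; On BeginPlay it gives the platform a random mesh from a StaticMesh array and spawns an effect system attached to that mesh.
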(event EventBeginPlay
  (Components|StaticMesh|SetStaticMesh (Variables|Default|GetSM_RockPlateForm) (Utilities|Array|Get(acopy) (Variables|Default|GetStaticMesh) (Math|Random|RandomIntegerinRange 0 5)))
  (Niagara|SpawnSystemAttached 0 (Variables|Default|GetSM_RockPlateForm) "None" (Transformation|GetActorLocation) (Transformation|GetActorRotation) "KeepWorldPosition" false))

(event Collision|EventActorBeginOverlap
  (params (OtherActor :type Actor%20Object%20Reference)))

(event EventTick
  (params (DeltaSeconds :type Float%20%28single-precision%29)))

(fn ConstructionScript
  (bind _interptomovement (Variables|Default|GetInterpToMovement))
  (Variables|/Script/Engine.InterpToMovementComponent|SetControlPoints _interptomovement (Utilities|Array|MakeArray (Utilities|Struct|MakeInterpControlPoint (Variables|Default|GetLoc1) true) (Utilities|Struct|MakeInterpControlPoint (Variables|Default|GetLoc2) true)))
  (Variables|/Script/Engine.InterpToMovementComponent|SetDuration _interptomovement (Variables|Default|GetDuration)))