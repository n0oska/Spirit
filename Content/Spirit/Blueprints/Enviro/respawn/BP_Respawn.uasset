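; BP_Respawn is a checkpoint trigger that records where the player respawns.
; When the first player's character overlaps its Box, it writes its own location and rotation into the BPGM_Spirit game mode.
; It also stores itself there as the last checkpoint, leaving the respawn itself to be handled outside this Blueprint.
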(event OnComponentBeginOverlap(Box)
  (params (OverlappedComponent :type Primitive%20Component%20Object%20Reference) (OtherActor :type Actor%20Object%20Reference) (OtherComp :type Primitive%20Component%20Object%20Reference) (OtherBodyIndex :type Integer) (bFromSweep :type Boolean) (SweepResult :type Hit%20Result%20Structure%20%28by%20ref%29))
  (if (== OtherActor (Game|GetPlayerCharacter 0))
    (bind _asbpgm_spirit (Utilities|Casting|CastToBPGM_Spirit (Game|GetGameMode)))
    (Variables|/Game/Spirit/Blueprints/Manager/BPGM_Spirit.BPGM_Spirit_C|SetActor%20Location _asbpgm_spirit (Transformation|GetActorLocation))
    (Variables|/Game/Spirit/Blueprints/Manager/BPGM_Spirit.BPGM_Spirit_C|SetActor%20Rotation _asbpgm_spirit (Transformation|GetActorRotation))
    (Variables|/Game/Spirit/Blueprints/Manager/BPGM_Spirit.BPGM_Spirit_C|SetLastCheckpoint _asbpgm_spirit self)))

(event EventBeginPlay)

(event Collision|EventActorBeginOverlap
  (params (OtherActor :type Actor%20Object%20Reference)))

(event EventTick
  (params (DeltaSeconds :type Float%20%28single-precision%29)))

(fn ConstructionScript)