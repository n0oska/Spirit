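; BP_RespawnManager returns the player character to a respawn point after death.
; On BeginPlay it caches the BP_Chara and BP_Respawn actors, each found by class lookup, so it works with a single respawn point.
; Its respawn event, not called within this Blueprint, checks the character's IsDead flag and, if set, moves it to the respawn actor's location and rotation without clearing the flag.
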(event Custom|respawn
  (bind _bp_chara (Variables|Default|GetBp_Chara))
  (bind _bp_respawn (Variables|Default|GetBP_respawn))
  (if (Variables|/Game/Spirit/Blueprints/Chara/BP_Chara.BP_Chara_C|GetIsDead _bp_chara)
    (Transformation|SetActorLocationAndRotation _bp_chara (Transformation|GetActorLocation _bp_respawn) (Transformation|GetActorRotation _bp_respawn))))

(event EventBeginPlay
  (bind _returnvalue (Actor|GetActorOfClass "/Game/Spirit/Blueprints/Chara/BP_Chara.BP_Chara_C"))
  (Variables|Default|SetBP_Chara _returnvalue)
  (bind _returnvalue_2 (Actor|GetActorOfClass "/Game/Spirit/Blueprints/Enviro/BP_Respawn.BP_Respawn_C"))
  (Variables|Default|SetBP_Respawn _returnvalue_2))

(fn ConstructionScript)