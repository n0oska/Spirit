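; BP_TPDepart is a teleport departure point that moves the BP_Chara character to an arrival point.
; At BeginPlay it caches the BP_Chara and BP_PointTpArrivée actors found through GetActorOfClass, so it assumes one of each.
; Any overlap with its Box calls TP, which teleports the character to the arrival point's location and rotation without checking which actor entered.
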(event OnComponentBeginOverlap(Box)
  (params (OverlappedComponent :type Primitive%20Component%20Object%20Reference) (OtherActor :type Actor%20Object%20Reference) (OtherComp :type Primitive%20Component%20Object%20Reference) (OtherBodyIndex :type Integer) (bFromSweep :type Boolean) (SweepResult :type Hit%20Result%20Structure%20%28by%20ref%29))
  (CallFunction|TP))

(event Custom|TP
  (bind _bp_pointtp (Variables|Default|GetBP_PointTP))
  (Transformation|SetActorLocationAndRotation (Variables|Default|GetBP_Chara) (Transformation|GetActorLocation _bp_pointtp) (Transformation|GetActorRotation _bp_pointtp) false true))

(event EventBeginPlay
  (bind _returnvalue (Actor|GetActorOfClass "/Game/Spirit/Blueprints/Chara/BP_Chara.BP_Chara_C"))
  (Variables|Default|SetBP_Chara _returnvalue)
  (bind _returnvalue_2 (Actor|GetActorOfClass "/Game/Spirit/Blueprints/Enviro/BP_PointTpArrivée.BP_PointTpArrivée_C"))
  (Variables|Default|SetBP_PointTP _returnvalue_2))

(event Collision|EventActorBeginOverlap
  (params (OtherActor :type Actor%20Object%20Reference)))

(event EventTick
  (params (DeltaSeconds :type Float%20%28single-precision%29)))

(fn ConstructionScript)