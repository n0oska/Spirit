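; LD_BP is a level-design building tool that procedurally assembles blocks of a chosen static mesh from X, Y and Z counts.
; The construction script rebuilds a HISM, spacing instances by the mesh's bounding box.
; ConstructionMode selects wall/tunnel (optionally hollowed or reduced to a frame), staircase, stacked rings set by Radius, or ramp.
; Ramp pieces are pitched by a clamped Inclinaison and stretched along X; the event graph is unused.
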(event EventBeginPlay)

(event Collision|EventActorBeginOverlap
  (params (OtherActor :type Actor%20Object%20Reference)))

(event EventTick
  (params (DeltaSeconds :type Float%20%28single-precision%29)))

(fn ConstructionScript
  (bind _inclinaison (Variables|Ramp|GetInclinaison))
  (bind _staticmesh (Variables|Default|GetStaticMesh))
  (bind _returnvalue (Math|Float|Clamp(Float) _inclinaison 0.0 35.0))
  (bind _returnvalue_2 (StaticMesh|GetBoundingBox _staticmesh))
  (bind _returnvalue_3 (- (.max _returnvalue_2) (.min _returnvalue_2)))
  (Components|InstancedStaticMesh|ClearInstances (Variables|Default|GetHISM))
  (if (Math|Boolean|ANDBoolean (> (Variables|Default|Getx) 0) (> (Variables|Default|Getz) 0) (> (Variables|Size|GetY) 0) (Utilities|IsValid (Variables|Default|GetStaticMesh)))
    (Components|StaticMesh|SetStaticMesh (Variables|Default|GetHISM) (Variables|Default|GetStaticMesh))
    (Variables|Default|SetX_SizeOfCube (.x _returnvalue_3))
    (Variables|Default|SetY_SizeOfCube (.y _returnvalue_3))
    (Variables|Default|SetZ_SizeOfCube (.z _returnvalue_3))
    (switch Utilities|FlowControl|Switch|SwitchonE_ConstructionMode (Variables|WhichForm?|GetConstructionMode)
      (:NewEnumerator0
        ;[0.15 0.15 0.15 0.5] Mur ou Cube/Cadre
        (for _index (range 0 (- (Variables|Size|GetX) 1))
          (LocalVariables|SetIndex_X _index)
          (for _index_2 (range 0 (- (Variables|Size|GetZ) 1))
            (LocalVariables|SetIndex_Z _index_2)
            (for _index_3 (range 0 (- (Variables|Size|GetY) 1))
              (LocalVariables|SetIndex_Y _index_3)
              (if (select (Variables|WhichForm?|GetTunnel) (or (or (== (LocalVariables|GetIndex_X) 0) (== (LocalVariables|GetIndex_X) (- (Variables|Size|GetX) 1))) (or (== (LocalVariables|GetIndex_Z) 0) (== (LocalVariables|GetIndex_Z) (- (Variables|Size|GetZ) 1)))) (Class|KismetSystemLibrary|MakeLiteralBool true))
                (if (select (Variables|WhichForm?|GetCadre) (Math|Boolean|ORBoolean (and (or (== (LocalVariables|GetIndex_Z) 0) (== (LocalVariables|GetIndex_Z) (- (Variables|Size|GetZ) 1))) (or (== (LocalVariables|GetIndex_Y) 0) (== (LocalVariables|GetIndex_Y) (- (Variables|Size|GetY) 1)))) (and (or (== (LocalVariables|GetIndex_Z) 0) (== (LocalVariables|GetIndex_Z) (- (Variables|Size|GetZ) 1))) (or (== (LocalVariables|GetIndex_X) 0) (== (LocalVariables|GetIndex_X) (- (Variables|Size|GetX) 1)))) (and (or (== (LocalVariables|GetIndex_X) 0) (== (LocalVariables|GetIndex_X) (- (Variables|Size|GetX) 1))) (or (== (LocalVariables|GetIndex_Y) 0) (== (LocalVariables|GetIndex_Y) (- (Variables|Size|GetY) 1))))) (Class|KismetSystemLibrary|MakeLiteralBool true))
                  (Components|InstancedStaticMesh|AddInstance (Variables|Default|GetHISM) (Math|Transform|MakeTransform (Math|Vector|MakeVector (* (LocalVariables|GetIndex_X) (Variables|Default|GetX_SizeOfCube)) (* (LocalVariables|GetIndex_Y) (Variables|Default|GetY_SizeOfCube)) (* (LocalVariables|GetIndex_Z) (Variables|Default|GetZ_SizeOfCube)))) false)))))))
      (:NewEnumerator1
        ;[0.15 0.15 0.15 0.5] Escalier
        (for _index_4 (range 0 (- (Variables|Size|GetX) 1))
          (LocalVariables|SetIndex_X _index_4)
          (for _index_5 (range 0 (- (- (Variables|Size|GetZ) 1) (LocalVariables|GetIndex_X)))
            (LocalVariables|SetIndex_Z _index_5)
            (for _index_6 (range 0 (- (Variables|Size|GetY) 1))
              (LocalVariables|SetIndex_Y _index_6)
              (Components|InstancedStaticMesh|AddInstance (Variables|Default|GetHISM) (Math|Transform|MakeTransform (Math|Vector|MakeVector (* (LocalVariables|GetIndex_X) (Variables|Default|GetX_SizeOfCube)) (* (LocalVariables|GetIndex_Y) (Variables|Default|GetY_SizeOfCube)) (* (LocalVariables|GetIndex_Z) (Variables|Default|GetZ_SizeOfCube)))) false)))))
      (:NewEnumerator2
        ;[0.15 0.15 0.15 0.5] Circle
        (for _index_7 (range 0 (- (Variables|Size|GetZ) 1))
          (LocalVariables|SetIndex_Z _index_7)
          (for _index_8 (range 0 (- (Variables|Size|GetX) 1))
            (LocalVariables|SetIndex_X _index_8)
            (Components|InstancedStaticMesh|AddInstance (Variables|Default|GetHISM) (Math|Transform|MakeTransform (+ (Math|Vector|MakeVector 0.0 0.0 (* (LocalVariables|GetIndex_Z) (Variables|Default|GetZ_SizeOfCube))) (Math|Vector|RotateVector (+ "" (* (Math|Vector|GetForwardVector (Math|Rotator|MakeRotator 0.0 0.0 (Math|Conversions|ToFloat(Integer) (* (LocalVariables|GetIndex_X) (/ 3.6e+02 (Math|Conversions|ToFloat(Integer) (Variables|Size|GetX))))))) (Variables|Ring|GetRadius))) (Variables|Ring|GetRotation))) (Math|Rotator|CombineRotators (Math|Conversions|RotationFromXVector (* (Math|Vector|GetForwardVector (Math|Rotator|MakeRotator 0.0 0.0 (Math|Conversions|ToFloat(Integer) (* (LocalVariables|GetIndex_X) (/ 3.6e+02 (Math|Conversions|ToFloat(Integer) (Variables|Size|GetX))))))) (Variables|Ring|GetRadius))) (Variables|Ring|GetRotation))) false))))
      (:NewEnumerator5
        ;[0.15 0.15 0.15 0.5] Ramp
        (for _index_9 (range 0 (- (Variables|Size|GetX) 1))
          (LocalVariables|SetIndex_X _index_9)
          (for _index_10 (range 0 (- (- (Variables|Size|GetZ) 1) (LocalVariables|GetIndex_X)))
            (LocalVariables|SetIndex_Z _index_10)
            (for _index_11 (range 0 (- (Variables|Size|GetY) 1))
              (LocalVariables|SetIndex_Y _index_11)
              (Components|InstancedStaticMesh|AddInstance (Variables|Default|GetHISM) (Math|Transform|MakeTransform (Math|Vector|MakeVector (* (LocalVariables|GetIndex_X) (Variables|Default|GetX_SizeOfCube)) (* (LocalVariables|GetIndex_Y) (Variables|Default|GetY_SizeOfCube)) (* (LocalVariables|GetIndex_X) _returnvalue)) (Math|Rotator|MakeRotator 1.0 _returnvalue 1.0) (Math|Vector|MakeVector (/ (Variables|Size|GetZ) (Math|Trig|Cos(Degrees) _returnvalue)) 1.0 1.0)) false))))))))